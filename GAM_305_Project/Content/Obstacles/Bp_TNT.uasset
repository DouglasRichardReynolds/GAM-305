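; TNT obstacle that explodes when the player's top-down character touches its capsule.
; The overlap enables query collision on the explosion radius, then loops over the actors inside it, with a short delay before applying damage, printing a debug message and destroying itself.
; Because the Delay sits inside the loop, it completes only once, so only the last actor in the array takes damage.
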(event `self.Capsule.OnComponentBeginOverlap`
  (params (OverlappedComponent :type "PrimitiveComponent Object Reference") (OtherActor :type "Actor Object Reference") (OtherComp :type "PrimitiveComponent Object Reference") (OtherBodyIndex :type Integer) (bFromSweep :type Boolean) (SweepResult :type "HitResult Structure (by ref)"))
  (bind _explosion_radius (`self.Explosion_radius`))
  (cast `/Game/TopDown/Blueprints/BP_TopDownCharacter` OtherActor)
  (`PrimitiveComponent.SetCollisionEnabled` _explosion_radius "QueryOnly")
  (for _array_element (`PrimitiveComponent.GetOverlappingActors` _explosion_radius null)
    (`KismetSystemLibrary.Delay` 0.5)
    (`GameplayStatics.ApplyDamage` _array_element 1.0 null self)
    (`KismetSystemLibrary.PrintString` "tnt exploide")
    (`self.K2_DestroyActor` self)))

(fn `UserConstructionScript`)