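; Player character for a shooter that moves relative to control yaw, rotates toward a supplied aim point and hops between Teleporter actors.
; Held fire spawns projectiles through a Gate and RetriggerableDelay loop paced by FireRate, alongside a leftover laser trace marked unused.
; Reported kills re-arm the DoOnce-guarded teleport at a threshold, and teleporting advances the index and clears the count.
; Armor absorbs one hit before death, with Player_W showing teleport and death overlays.
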(event `InputAction|Shoot`
  (params (Key :type "Key Structure"))
  (bind _cube (`self.Cube`))
  ;[1 1 1] Laser (Unused)
  (:`Pressed`
    (`KismetSystemLibrary.LineTraceSingle` (`SceneComponent.K2_GetComponentLocation` _cube) (* (`SceneComponent.GetForwardVector` _cube) 10000.0) "TraceTypeQuery1")))

(event `InputAction|Teleport`
  (params (Key :type "Key Structure"))
  ;[1 1 1] Teleport
  (:`Pressed`
    (`/Engine/EditorBlueprintResources/StandardMacros.DoOnce` false :!label _label
      (:`Completed`
        (`self.GoToTeleporter`)
        (set `self.KillCount` 0)
        (`/Game/Player/Player_W.DisableTPOverlay` (`self.PlayerWidget`))))))

(event `ResetTeleporter`
  ;[1 1 1] Teleport
  (goto _label :!via `Reset`))

(event `AddKill`
  (bind _killcount (`self.KillCount`))
  ;[1 1 1] Count Kill & Reset Teleporter
  (set `self.KillCount` (+ _killcount 1))
  (if (>= _killcount 4)
    (`self.ResetTeleporter`)
    (`/Game/Player/Player_W.EnableTPOverlay` (`self.PlayerWidget`))))

(event `GoToTeleporter`
  ;[1 1 1] Teleport
  (`self.K2_SetActorLocation` (`self.K2_GetActorLocation` (`|GetArrayItem` (`self.Teleporters`) (`self.CurrentTeleporter`))))
  (set `self.CurrentTeleporter` (+ (`self.CurrentTeleporter`) 1)))

(event `self.ReceiveBeginPlay`
  (bind _outactors (`GameplayStatics.GetAllActorsOfClass` "/Game/Player/Teleporter.Teleporter_C"))
  (set `self.Teleporters` _outactors)
  (bind _returnvalue (`|CreateWidget` "/Game/Player/Player_W.Player_W_C"))
  (set `self.PlayerWidget` _returnvalue)
  (`UserWidget.AddToViewport` _returnvalue 0))

(event `InputAxis|MovementY`
  (params (AxisValue :type "Float (single-precision)"))
  (bind (_returnvalue_roll _returnvalue_pitch _returnvalue_yaw) (`KismetMathLibrary.BreakRotator` (`self.GetControlRotation`)))
  ;[1 1 1] Movement
  (`self.AddMovementInput` (`KismetMathLibrary.GetForwardVector` (`KismetMathLibrary.MakeRotator` 0.0 0.0 _returnvalue_yaw)) AxisValue))

(event `InputAction|Shoot`
  (params (Key :type "Key Structure"))
  ;[1 1 1] Shoot
  (:`Pressed`
    (`/Engine/EditorBlueprintResources/StandardMacros.DoOnce` false :!label _label_2
      (:`Completed`
        (`|ExecutionSequence`
          (:`then_0`
            (goto _label_3 :!via `Open`))
          (:`then_1`
            (`/Engine/EditorBlueprintResources/StandardMacros.Gate` true :!label _label_3
              (:`Exit`
                (`|ExecutionSequence`
                  (:`then_0`
                    (`self.ShootProjectile`))
                  (:`then_1`
                    (`KismetSystemLibrary.RetriggerableDelay` (`self.FireRate`))
                    (`|ExecutionSequence`
                      (:`then_0`
                        (goto _label_3))
                      (:`then_1`
                        (goto _label_2 :!via `Reset`))))))))))))
  (:`Released`
    (goto _label_3 :!via `Close`)))

(event `ShootProjectile`
  (bind (_returnvalue_location _returnvalue_rotation _returnvalue_scale) (`KismetMathLibrary.BreakTransform` (`SceneComponent.K2_GetComponentToWorld` (`self.Arrow1`))))
  ;[1 1 1] Shoot
  (`|SpawnActorFromClass` "/Game/Player/PlayerProj_BP.PlayerProj_BP_C" (`KismetMathLibrary.MakeTransform` _returnvalue_location _returnvalue_rotation _returnvalue_scale) "Undefined" "MultiplyWithRoot" self null))

(event `InputAxis|MovementX`
  (params (AxisValue :type "Float (single-precision)"))
  (bind (_returnvalue_roll _returnvalue_pitch _returnvalue_yaw) (`KismetMathLibrary.BreakRotator` (`self.GetControlRotation`)))
  ;[1 1 1] Movement
  (`self.AddMovementInput` (`KismetMathLibrary.GetRightVector` (`KismetMathLibrary.MakeRotator` _returnvalue_roll 0.0 _returnvalue_yaw)) AxisValue))

(event `self.ReceiveAnyDamage`
  (params (Damage :type "Float (single-precision)") (DamageType :type "DamageType Object Reference") (InstigatedBy :type "Controller Object Reference") (DamageCauser :type "Actor Object Reference"))
  ;[1 1 1] Take Damage
  (if (`self.Armor`)
    (set `self.Armor` false)
    (else
      (`self.K2_DestroyActor`)
      (`/Game/Player/Player_W.EnableDeathOverlay` (`self.PlayerWidget`)))))

(event `/Game/Player/PlayerChar_BPI.LookAt`
  (params (Target :type "Vector Structure"))
  (bind (_returnvalue_x _returnvalue_y) (`KismetMathLibrary.BreakVector` (`self.K2_GetActorLocation`)))
  ;[1 1 1] Aim
  (`self.K2_SetActorRotation` (`KismetMathLibrary.FindLookAtRotation` (`KismetMathLibrary.MakeVector` _returnvalue_x _returnvalue_y) (`KismetMathLibrary.MakeVector` Target_X Target_Y))))

(fn `NewFunction`)

(fn `UserConstructionScript`)