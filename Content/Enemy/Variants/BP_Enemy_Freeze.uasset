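; BP_Enemy_Freeze is an enemy variant that moves to the player's location via AI MoveTo when Find_Player fires and SeesPlayer is true.
; AnyDamage subtracts from Health, calls an empty CheckHealth and prints the remaining value; TrackPlayer is also empty.
; Its hit handler spawns a SpeedUp actor at its own transform, but binds only from within itself, and no freeze logic appears here.
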(event `Find_Player`
  (bind _returnvalue_location (`KismetMathLibrary.BreakTransform` (`self.GetTransform` (`GameplayStatics.GetPlayerCharacter` 0))))
  (if (`self.SeesPlayer`)
    (`|AIMoveTo` null _returnvalue_location null)))

(event `self.ReceiveAnyDamage`
  (params (Damage :type "Float (single-precision)") (DamageType :type "DamageType Object Reference") (InstigatedBy :type "Controller Object Reference") (DamageCauser :type "Actor Object Reference"))
  (set `self.Health` (- (`self.Health`) Damage))
  (`self.CheckHealth`)
  (`KismetSystemLibrary.PrintString` (`KismetStringLibrary.Conv_DoubleToString` (`self.Health`)) true true (struct :`R` 0.963542 :`B` 0.062638 :`A` 1.0) 10.0))

(event `OnActorHit_Event` :!signature `self.OnActorHit`
  (params (SelfActor :type "Actor Object Reference") (OtherActor :type "Actor Object Reference") (NormalImpulse :type "Vector Structure") (Hit :type "HitResult Structure (by ref)"))
  (add `self.OnActorHit` (delegate `OnActorHit_Event`))
  (`|SpawnActorFromClass` "/Game/Powerups/SpeedUp.SpeedUp_C" (`self.GetTransform` SelfActor) "Undefined" "MultiplyWithRoot" null null))

(fn `CheckHealth`)

(fn `Track_player`)

(fn `UserConstructionScript`)